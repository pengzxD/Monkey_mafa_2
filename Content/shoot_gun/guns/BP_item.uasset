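; BP_item is an item Blueprint that shows an interaction widget while a player is in interaction range.
; On range enter, it creates an Interactiion widget for the player's controller and adds a widget component, stored to prevent duplicates, though no link between the two is shown.
; On range exit, it destroys that component.
; GetInteractionText returns a fixed "interact" label, but the widget is created with empty text.
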(event EventOnInteractionRangeExit
  (bind _interaction_wiget (Variables|Default|Getinteraction%20wiget)
    (:then
      (Components|DestroyComponent _interaction_wiget))
    (:else)))

(event EventOnInteractionRangeEnterd
  (params (player :type Third%20Person%20Character%20Object%20Reference))
  (Variables|Default|Getinteraction%20wiget
    (:then)
    (:else
      (UserInterface|CreateWidget "/Game/shoot_gun/interactiion.interactiion_C" (.AsPlayer%20Controller (Utilities|Casting|CastToPlayerController (Pawn|GetController player))))
      (bind _returnvalue (AddComponent|AddWidgetComponent false))
      (Variables|Default|Setinteraction%20wiget _returnvalue))))

(fn ConstructionScript)

(fn GetInteractionText
  (return "interact"))